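; WareWolf is a 2D flipbook enemy that patrols, chases and attacks the player, and drops a gold coin on death.
; Tick drives movement, animation, death and sound only while the camera is vertically near.
; Overlap volumes turn it around, trigger faster chasing and start randomly chosen attacks, which damage and knock back the player on a specific animation frame.
; Shuriken and sword hits tint it and reduce health; health bar logic is disconnected.
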(event OnComponentEndOverlap(RotatingBox)
  (params (OverlappedComponent :type Primitive%20Component%20Object%20Reference) (OtherActor :type Actor%20Object%20Reference) (OtherComp :type Primitive%20Component%20Object%20Reference) (OtherBodyIndex :type Integer))
  ;[1 1 1] Rotating
  (Transformation|SetActorRotation (Math|Rotator|CombineRotators (Transformation|GetActorRotation) "0.000000,180.000000,0.000000")))

(event OnComponentBeginOverlap(AttackingChase)
  (params (OverlappedComponent :type Primitive%20Component%20Object%20Reference) (OtherActor :type Actor%20Object%20Reference) (OtherComp :type Primitive%20Component%20Object%20Reference) (OtherBodyIndex :type Integer) (bFromSweep :type Boolean) (SweepResult :type Hit%20Result%20Structure%20%28by%20ref%29))
  ;[1 1 1] Detecting Character
  (bind _ascharacter_bp (Utilities|Casting|CastToCharacter_Bp OtherActor))
  (Variables|Default|SetAs%20Character%20Bp _ascharacter_bp)
  (Variables|Default|SetcharacterDetected true)
  (Variables|/Script/Engine.CharacterMovementComponent|SetMaxWalkSpeed (Variables|Character|GetCharacterMovement) 2e+02))

(event OnComponentEndOverlap(AttackingChase)
  (params (OverlappedComponent :type Primitive%20Component%20Object%20Reference) (OtherActor :type Actor%20Object%20Reference) (OtherComp :type Primitive%20Component%20Object%20Reference) (OtherBodyIndex :type Integer))
  ;[1 1 1] Detecting Character
  (Utilities|Casting|CastToCharacter_Bp OtherActor)
  (Variables|Default|SetcharacterDetected false)
  (Variables|/Script/Engine.CharacterMovementComponent|SetMaxWalkSpeed (Variables|Character|GetCharacterMovement) 1e+02)
  (CallFunction|ResetWareWolfSound))

(event OnComponentBeginOverlap(CapsuleComponent)
  (params (OverlappedComponent :type Primitive%20Component%20Object%20Reference) (OtherActor :type Actor%20Object%20Reference) (OtherComp :type Primitive%20Component%20Object%20Reference) (OtherBodyIndex :type Integer) (bFromSweep :type Boolean) (SweepResult :type Hit%20Result%20Structure%20%28by%20ref%29))
  ;[1 1 1] Shuriken Damage
  (Utilities|Casting|CastToShuriken1 OtherActor)
  (Audio|PlaySound2D "/Game/Music/ShurikenDamageSound/ShurikenDmageSound.ShurikenDmageSound" 1.0 1.0 0.0 0 0)
  (Variables|Default|Sethealth (- (Variables|Default|Gethealth) 1.0))
  (Variables|Default|SetWareWolfHurting true)
  (Sprite|SetSpriteColor (Variables|Default|GetWareWolf_Ideal) "(R=0.527115,G=0.000000,B=0.019382,A=1.000000)")
  (Utilities|FlowControl|Delay 0.2)
  (Sprite|SetSpriteColor (Variables|Default|GetWareWolf_Ideal) "(R=1.000000,G=0.906830,B=0.948081,A=1.000000)")
  (Variables|Default|SetWareWolfHurting false))

(event OnComponentBeginOverlap(AttackDetection)
  (params (OverlappedComponent :type Primitive%20Component%20Object%20Reference) (OtherActor :type Actor%20Object%20Reference) (OtherComp :type Primitive%20Component%20Object%20Reference) (OtherBodyIndex :type Integer) (bFromSweep :type Boolean) (SweepResult :type Hit%20Result%20Structure%20%28by%20ref%29))
  ;[1 1 1] Chasing For Attack
  (bind _ascharacter_bp (Utilities|Casting|CastToCharacter_Bp OtherActor))
  (Variables|Default|SetAs%20Character%20Bp_1 _ascharacter_bp)
  (CallFunction|GenerateNumber)
  (Variables|Default|SetIsOverlapping true))

(event OnComponentEndOverlap(AttackDetection)
  (params (OverlappedComponent :type Primitive%20Component%20Object%20Reference) (OtherActor :type Actor%20Object%20Reference) (OtherComp :type Primitive%20Component%20Object%20Reference) (OtherBodyIndex :type Integer))
  ;[1 1 1] Chasing For Attack
  (Utilities|Casting|CastToCharacter_Bp OtherActor)
  (Variables|Default|SetIsOverlapping false))

(event Custom|Get%20player%20rotation
  (bind _capsulecomponent (Variables|Collision|GetCapsuleComponent))
  ;[1 1 1] Chasing Character and rotating
  (Utilities|IsValid (Variables|Default|GetAs%20Character%20Bp)
    (:Is%20Valid
      (if (Variables|Default|GetcharacterDetected)
        (Variables|Default|Setrunning true)
        (Math|Float|CompareFloat (- (.x (Transformation|GetActorLocation)) (.x (Transformation|GetActorLocation (Variables|Default|GetAs%20Character%20Bp)))) 0.0
          (:>
            (Transformation|SetWorldRotation _capsulecomponent "0.000000,-180.000000,0.000000" false false))
          (:<
            (Transformation|SetWorldRotation _capsulecomponent "0, 0, 0" false false)))
        (CallFunction|Attack)
        (else
          (Variables|Default|Setrunning false))))))

(event Custom|Attack
  ;[1 1 1] WareWolf Attack
  (if (Variables|Default|GetIsOverlapping)
    (if (not (Variables|/Game/MainCharacter/Character_Bp.Character_Bp_C|GetHealth%20Boost%20Power (Variables|Default|GetAs%20Character%20Bp)))
      (if (== (Class|PaperFlipbookComponent|GetPlaybackPositioninFrames (Variables|Default|GetWareWolf_Ideal)) 5)
        (Utilities|FlowControl|DoOnce false
          (:Completed
            (Audio|PlaySound2D "/Game/Music/Hurting/MainCharacterHuring/femalehurtingsound_Cue.femalehurtingsound_Cue" 1.0 1.0 0.0 0 0)
            (Game|Feedback|ClientPlayForceFeedback (Game|GetPlayerController 0) "/Game/HapticFeedBack/Damage.Damage" "None" false false false)
            (bind _result (Math|Integer|DecrementInt (Variables|/Game/MainCharacter/Character_Bp.Character_Bp_C|Gethealth (Variables|Default|GetAs%20Character%20Bp_1)))
              (:%20%20
                (Variables|/Game/MainCharacter/Character_Bp.Character_Bp_C|Sethealth (Variables|Default|GetAs%20Character%20Bp_1) _result)
                (Utilities|FlowControl|Sequence
                  (:then_0
                    (Sprite|SetSpriteColor (Variables|/Game/MainCharacter/Character_Bp.Character_Bp_C|GetIdle (Variables|Default|GetAs%20Character%20Bp_1)) "(R=0.526042,G=0.000000,B=0.019498,A=1.000000)")
                    (CallFunction|HitBack))
                  (:then_1
                    (Utilities|FlowControl|Delay 0.8)
                    (CallFunction|ResetColorChange)))))))))))

(event Custom|Animation
  ;[1 1 1] Animation
  (if (Variables|Default|Getisdead)
    (Sprite|SetFlipbook (Variables|Default|GetWareWolf_Ideal) "/Game/images/Enemies/WareWolf/WareWolfDead.WareWolfDead")
    (else
      (Sprite|SetFlipbook (Variables|Default|GetWareWolf_Ideal) (select (== (Variables|/Script/Engine.CharacterMovementComponent|GetMaxWalkSpeed (Variables|Character|GetCharacterMovement)) 0.0) "/Game/images/Enemies/WareWolf/WareWolf_Ideal.WareWolf_Ideal" (select (and (== (Variables|Default|GetsetNumber) 1) (Variables|Default|GetIsOverlapping)) "/Game/images/Enemies/WareWolf/WareWolf_Attack1.WareWolf_Attack1" (select (and (== (Variables|Default|GetsetNumber) 0) (Variables|Default|GetIsOverlapping)) "/Game/images/Enemies/WareWolf/WareWolf_RunAttack.WareWolf_RunAttack" (select (Variables|Default|Getrunning) (select (Variables|Default|GetcharacterDetected) "/Game/images/Enemies/WareWolf/WareWolf_Run.WareWolf_Run" "/Game/images/Enemies/WareWolf/WareWolf_Walk.WareWolf_Walk") "/Game/images/Enemies/WareWolf/WareWolf_Walk.WareWolf_Walk"))))))))

(event Custom|GenerateNumber
  ;[1 1 1] Generate Random Number For Attack Animation
  (Variables|Default|SetsetNumber (Math|Random|RandomInteger 2)))

(event Custom|WareWolfDamageHurting
  (bind _warewolf_ideal (Variables|Default|GetWareWolf_Ideal))
  (bind _warewolf_ideal_2 (Variables|Default|GetWareWolf_Ideal))
  (bind _returnvalue (Transformation|GetWorldTransform _warewolf_ideal))
  (bind _returnvalue_2 (Transformation|GetWorldTransform _warewolf_ideal_2))
  ;[1 1 1] WareWolfHurtingAnimation
  (if (Variables|Default|GetWareWolfHurting)
    (Transformation|SetWorldTransform (Variables|Default|GetWareWolf_Ideal) (Math|Transform|MakeTransform (.location _returnvalue) (Math|Rotator|MakeRotator (.roll (.rotation _returnvalue)) -5.0 (.yaw (.rotation _returnvalue))) (.scale _returnvalue)) false false)
    (Sprite|SetFlipbook (Variables|Default|GetWareWolf_Ideal) "/Game/images/Enemies/WareWolf/WareWolfHurt.WareWolfHurt")
    (Components|Activation|Deactivate (Variables|Character|GetCharacterMovement))
    (Utilities|FlowControl|Delay 0.5)
    (Transformation|SetWorldTransform (Variables|Default|GetWareWolf_Ideal) (Math|Transform|MakeTransform (.location _returnvalue_2) (Math|Rotator|MakeRotator (.roll (.rotation _returnvalue_2)) 15.0 (.yaw (.rotation _returnvalue_2))) (.scale _returnvalue_2)) false false)
    (Components|Activation|Activate (Variables|Character|GetCharacterMovement) false)))

(event Custom|WareWolfSound
  ;[1 1 1] Sound
  (if (Variables|Default|GetcharacterDetected)
    (Utilities|FlowControl|DoOnce false
      (:Completed
        (Audio|Components|Audio|SetSound (Variables|Default|Getwarewolfattak) "/Game/Music/WareWolfAttack/warewolfattak.warewolfattak")
        (Audio|Components|Audio|Play (Variables|Default|Getwarewolfattak) 0.0)))
    (else
      (Audio|Components|Audio|FadeOut (Variables|Default|Getwarewolfattak) 2.0 5e+01 "Linear" :!class /Script/Engine.AudioComponent)
      (Audio|Components|Audio|Stop (Variables|Default|Getwarewolfattak)))))

(event Custom|HitBack
  (bind _as_character_bp_1 (Variables|Default|GetAs%20Character%20Bp_1))
  ;[1 1 1] HitBack
  (if (== 1.8e+02 (.yaw (Transformation|GetWorldRotation (Variables|/Game/MainCharacter/Character_Bp.Character_Bp_C|GetIdle (Variables|Default|GetAs%20Character%20Bp_1)))))
    (Utilities|FlowControl|DoOnce false
      (:Completed
        (Character|LaunchCharacter _as_character_bp_1 "500.000000,0.000000,50.000000" false false)))
    (else
      (Utilities|FlowControl|DoOnce false
        (:Completed
          (Character|LaunchCharacter _as_character_bp_1 "-500.000000,0.000000,50.000000" false false)))))
  (Variables|/Game/MainCharacter/Character_Bp.Character_Bp_C|Setishurting (Variables|Default|GetAs%20Character%20Bp_1) true)
  (Utilities|FlowControl|Delay 0.2)
  (Sprite|SetSpriteColor (Variables|/Game/MainCharacter/Character_Bp.Character_Bp_C|GetIdle (Variables|Default|GetAs%20Character%20Bp_1)) "(R=1.000000,G=0.992634,B=0.970537,A=1.000000)")
  (Variables|/Game/MainCharacter/Character_Bp.Character_Bp_C|Setishurting (Variables|Default|GetAs%20Character%20Bp_1) false)
  (CallFunction|HitBackReset))

(event Custom|HitBack%20Reset
  (bind _as_character_bp_1 (Variables|Default|GetAs%20Character%20Bp_1))
  ;[1 1 1] HitBack
  (Utilities|FlowControl|Sequence
    (:then_0
      (Utilities|FlowControl|DoOnce false) ; enters at Reset
    )
    (:then_1
      (Utilities|FlowControl|DoOnce false) ; enters at Reset
    )))

(event Custom|Reset%20Color%20Change
  ;[1 1 1] WareWolf Attack
  (Utilities|FlowControl|DoOnce false) ; enters at Reset
)

(event Custom|HealthBarWareWolf
  ;[1 1 1] Health Bar
)

(event Custom|SitDetection)

(event Custom|ResetWareWolfSound
  ;[1 1 1] Sound
  (Utilities|FlowControl|DoOnce false) ; enters at Reset
)

(event Custom|Sword%20Attack%20on%20WareWolf
  ;[1 1 1] Sword Attack on WareWolf
  (Variables|Default|Sethealth (- (Variables|Default|Gethealth) 5.0))
  (Sprite|SetSpriteColor (Variables|Default|GetWareWolf_Ideal) "(R=1.000000,G=0.025124,B=0.000000,A=1.000000)")
  (Variables|Default|SetWareWolfHurting true)
  (Utilities|FlowControl|Delay 0.5)
  (Sprite|SetSpriteColor (Variables|Default|GetWareWolf_Ideal) "(R=1.000000,G=0.953415,B=0.974041,A=1.000000)")
  (Variables|Default|SetWareWolfHurting false))

(event Custom|Death
  (bind _warewolf_ideal (Variables|Default|GetWareWolf_Ideal))
  (bind _returnvalue (Transformation|GetWorldTransform _warewolf_ideal))
  ;[1 1 1] Death
  (if (<= (Variables|Default|Gethealth) 0.0)
    (Variables|Default|Setisdead true)
    (Components|Activation|Deactivate (Variables|Character|GetCharacterMovement))
    (Transformation|SetWorldTransform (Variables|Default|GetWareWolf_Ideal) (Math|Transform|MakeTransform (.location _returnvalue) (Math|Rotator|MakeRotator (.roll (.rotation _returnvalue)) -5.0 (.yaw (.rotation _returnvalue))) (.scale _returnvalue)) false false)
    (Utilities|FlowControl|Delay 1.0)
    (Game|SpawnActorfromClass "/Game/Collectables_and_PowerUps/GoldcOIN.GoldcOIN_C" (Transformation|GetWorldTransform (Variables|Collision|GetCapsuleComponent)) "Undefined" "MultiplyWithRoot" 0 0)
    (Actor|DestroyActor)
    (else
      (Variables|Default|Setisdead false)
      (CallFunction|GetPlayerRotation)
      (CallFunction|WareWolfDamageHurting))))

(event EventTick
  (params (DeltaSeconds :type Float%20%28single-precision%29))
  (bind _returnvalue (Game|GetPlayerCameraManager 0))
  (bind _returnvalue_2 (Transformation|GetActorLocation))
  (bind _returnvalue_3 (Camera|GetCameraLocation _returnvalue))
  (bind _returnvalue_4 (- (.z _returnvalue_3) (.z _returnvalue_2)))
  ;[1 1 1] WareWolf Movement
  (if (and (<= _returnvalue_4 5e+02) (>= _returnvalue_4 -5e+02))
    (CallFunction|Animation)
    (CallFunction|Death)
    (Pawn|Input|AddMovementInput (Transformation|GetActorForwardVector) 1.0 false)
    (CallFunction|HealthBarWareWolf)
    (CallFunction|WareWolfSound)
    (CallFunction|SitDetection)))

(fn ConstructionScript)