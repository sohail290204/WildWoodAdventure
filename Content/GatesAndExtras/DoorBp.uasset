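; Paper2D door gate that lets the player through on pressing G in its Purchase overlap zone with enough coin.
; Overlap events set the character's range flag and prompt text; the purchase check disables Block collision and sets DoorOpen, without deducting coins here.
; Tick picks the flipbook from DoorOpen and End, stopping at frame 4, where it runs that check.
; Block collision is restored past a hardcoded player X position.
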(event OnComponentBeginOverlap(purchase)
  (params (OverlappedComponent :type Primitive%20Component%20Object%20Reference) (OtherActor :type Actor%20Object%20Reference) (OtherComp :type Primitive%20Component%20Object%20Reference) (OtherBodyIndex :type Integer) (bFromSweep :type Boolean) (SweepResult :type Hit%20Result%20Structure%20%28by%20ref%29))
  ;[1 1 1] Plyer IN Range
  (bind _ascharacter_bp (Utilities|Casting|CastToCharacter_Bp OtherActor))
  (bind _output_get (Variables|Default|SetAs%20Character%20Bp _ascharacter_bp))
  (Variables|/Game/MainCharacter/Character_Bp.Character_Bp_C|SetpurchaseRange _output_get true)
  (if (not (Variables|Default|Getdoor%20Open))
    (Variables|Default|SettextMsg "Need 1 Coin to pass the door")))

(event OnComponentEndOverlap(purchase)
  (params (OverlappedComponent :type Primitive%20Component%20Object%20Reference) (OtherActor :type Actor%20Object%20Reference) (OtherComp :type Primitive%20Component%20Object%20Reference) (OtherBodyIndex :type Integer))
  ;[1 1 1] Plyer IN Range
  (bind _ascharacter_bp (Utilities|Casting|CastToCharacter_Bp OtherActor))
  (Variables|/Game/MainCharacter/Character_Bp.Character_Bp_C|SetpurchaseRange _ascharacter_bp false)
  (Variables|Default|SettextMsg ""))

(event Custom|Purchase%20Range
  (bind _as_character_bp (Variables|Default|GetAs%20Character%20Bp))
  ;[1 1 1] Display Message
  (CallFunction|PlayerLocation)
  (Utilities|IsValid _as_character_bp
    (:Is%20Valid
      (if (Variables|/Game/MainCharacter/Character_Bp.Character_Bp_C|GetpurchaseRange _as_character_bp)
        (if (Variables|/Game/MainCharacter/Character_Bp.Character_Bp_C|GetPressedG (Variables|Default|GetAs%20Character%20Bp))
          (if (Variables|/Game/MainCharacter/Character_Bp.Character_Bp_C|GetEnoughCoin (Variables|Default|GetAs%20Character%20Bp))
            (Collision|SetCollisionEnabled (Variables|Default|Getblock) "NoCollision")
            (Variables|Default|Setdoor%20Open true)
            (else
              (Variables|Default|SettextMsg "You dont have enough coin Need One Coin to Enter")
              (Variables|Default|Setdoor%20Open false))))
        (else
          (Variables|Default|SettextMsg ""))))))

(event Custom|PlayerLocation
  (bind _returnvalue (Actor|GetActorOfClass "/Game/MainCharacter/Character_Bp.Character_Bp_C"))
  (bind _output_get (Variables|Default|SetCharacterRef _returnvalue))
  (if (<= (.x (Transformation|GetActorLocation _output_get)) -3838.0)
    (Development|PrintString "Hello")
    (Collision|SetCollisionEnabled (Variables|Default|Getblock) "QueryAndPhysics")))

(event EventTick
  (params (DeltaSeconds :type Float%20%28single-precision%29))
  ;[1 1 1] Animation
  (Sprite|SetFlipbook (Variables|Default|GetDoor_1) (select (Variables|Default|Getdoor%20Open) 0 (select (Variables|Default|Getend) 0 0)))
  ;[1 1 1] Stop At that Frame of Animation
  (if (== (Class|PaperFlipbookComponent|GetPlaybackPositioninFrames (Variables|Default|GetDoor_1)) 4)
    (Audio|Components|Audio|Stop (Variables|Default|GetDoor_1))
    (CallFunction|PurchaseRange)))

(fn ConstructionScript)