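; Exploding tile hazard that shows a paper tilemap, set on BeginPlay, and blows up shortly after a Character_Bp touches it.
; Box overlap starts a short delay, then spawns an explosion emitter, plays a 2D blast sound and destroys the actor.
; Independently of overlap, chained Delays on Tick make the tilemap color alternate between red and near-white as a repeating flash.
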(event OnComponentBeginOverlap(Box)
  (params (OverlappedComponent :type Primitive%20Component%20Object%20Reference) (OtherActor :type Actor%20Object%20Reference) (OtherComp :type Primitive%20Component%20Object%20Reference) (OtherBodyIndex :type Integer) (bFromSweep :type Boolean) (SweepResult :type Hit%20Result%20Structure%20%28by%20ref%29))
  (Utilities|Casting|CastToCharacter_Bp OtherActor)
  (Utilities|FlowControl|Delay 0.8)
  (Effects|SpawnEmitteratLocation "/Game/StarterContent/Particles/P_Explosion.P_Explosion" "0, 0, 0" "0, 0, 0" "1.000000,1.000000,0.000000" true "ManualRelease")
  (Audio|PlaySound2D "/Game/Music/Exploding/blast-37988_Cue.blast-37988_Cue" 1.0 1.0 0.0 0 0)
  (Actor|DestroyActor))

(event EventBeginPlay
  (Class|PaperTileMapComponent|SetTileMap (Variables|Default|GetPaperTileMap) (Variables|Default|Gettilemap)))

(event Collision|EventActorBeginOverlap
  (params (OtherActor :type Actor%20Object%20Reference)))

(event EventTick
  (params (DeltaSeconds :type Float%20%28single-precision%29))
  (Utilities|FlowControl|Delay 0.5)
  (Class|PaperTileMapComponent|SetTileMapColor (Variables|Default|GetPaperTileMap) "(R=1.000000,G=0.058806,B=0.009047,A=1.000000)")
  (Utilities|FlowControl|Delay 0.8)
  (Class|PaperTileMapComponent|SetTileMapColor (Variables|Default|GetPaperTileMap) "(R=0.906830,G=0.958749,B=1.000000,A=1.000000)"))

(fn ConstructionScript)